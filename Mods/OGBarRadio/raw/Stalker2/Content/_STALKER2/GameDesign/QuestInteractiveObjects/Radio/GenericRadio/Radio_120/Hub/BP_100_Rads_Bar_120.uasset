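; Radio quest object variant for the 100 Rads Bar that plays the bar's sound cue when the player is nearby.
; Tick checks player distance and, in range, lazily spawns the cue on a newly added scene component, storing it as AudioComp.
; An existing sound resumes in range only while interaction is active, and pauses once the player leaves range, keeping its playback position.
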(event EventBeginPlay
  (|CallParentFunction) ; This node is disabled and will not be called.\nDrag off pins to build functionality.
)

(event Collision|EventActorBeginOverlap
  (params (OtherActor :type Actor%20Object%20Reference)))

(event EventTick
  (params (DeltaSeconds :type Float%20%28single-precision%29))
  (bind _returnvalue (Utilities|IsPlaying))
  (if (Utilities|IsWithinRange) ; isWithinRange
    (if (Utilities|IsValid (Variables|Default|GetAudioComp)) ; isAlive
      (if (Class|InteractableObject|IsInteractionActive) ; isActive
        (if (not _returnvalue) ; isPlaying
          (Class|AudioComponent|SetPaused (Variables|Default|GetAudioComp) false)))
      (else
        (bind _returnvalue_2 (CallFunction|CreateSound))
        (Variables|Default|SetAudioComp _returnvalue_2)))
    (elif true ; isAlive
      (if _returnvalue ; isPlaying
        (Class|AudioComponent|SetPaused (Variables|Default|GetAudioComp) true)))))

(fn ConstructionScript
  (|CallParentFunction))

(fn CreateSound
  (bind _returnvalue (AddComponent|AddSceneComponent false))
  (bind _returnvalue_2 (Audio|SpawnSoundAttached "/OGBarRadio/_STALKER2/GameDesign/QuestInteractiveObjects/Radio/GenericRadio/Radio_120/Hub/100_Rad_bar__SFX__Cue.100_Rad_bar__SFX__Cue" _returnvalue "None" "0, 0, 0" "0, 0, 0" "KeepRelativeOffset" true 0.75 1.0 0.0 "/OGBarRadio/_STALKER2/GameDesign/QuestInteractiveObjects/Radio/GenericRadio/Radio_120/Hub/NewSoundAttenuation.NewSoundAttenuation" 0 false))
  (return _returnvalue_2))